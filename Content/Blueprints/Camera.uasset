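; Camera rig Blueprint that turns with controller yaw and pitch input events.
; Yaw input rotates the whole actor, while pitch input rotates the SpringArmBackForth spring arm, clamped symmetrically by CameraPitchMax.
; CalculateResistance applies a cosine curve, scaled by ResistanceFactor, that slows pitch to zero toward the limits and speeds it up when returning toward level.
; The resistance value is also printed on screen.
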(event Custom|Controller%20Pitch%20Input
  (params (Value :type Float%20%28double-precision%29))
  (bind _springarm_backforth (Variables|Default|GetSpringArm_BackForth))
  (bind _returnvalue (Transformation|GetWorldRotation _springarm_backforth))
  (bind _resistance (CallFunction|CalculateResistance Value))
  (Transformation|SetWorldRotation _springarm_backforth (Math|Rotator|MakeRotator (.roll _returnvalue) (Math|Float|Clamp(Float) (- (.pitch _returnvalue) (* (* _resistance (Variables|Default|GetResistance%20Factor)) Value)) (* (Variables|Default|GetCamera%20Pitch%20Max) -1.0) (Variables|Default|GetCamera%20Pitch%20Max)) (.yaw _returnvalue)) false false))

(event Custom|Controller%20Yaw%20Input
  (params (Value :type Float%20%28double-precision%29))
  (bind _returnvalue (Transformation|GetActorRotation))
  (Transformation|SetActorRotation (Math|Rotator|MakeRotator (.roll _returnvalue) (.pitch _returnvalue) (+ Value (.yaw _returnvalue)))))

(event EventBeginPlay)

(event Collision|EventActorBeginOverlap
  (params (OtherActor :type Actor%20Object%20Reference)))

(event EventTick
  (params (DeltaSeconds :type Float%20%28single-precision%29)))

(fn ConstructionScript)

(fn CalculateResistance
  (params (Input :type Float%20%28double-precision%29))
  (bind _returnvalue (Math|Trig|GetPI))
  (bind _returnvalue_2 (Math|Trig|GetPI))
  (bind _springarm_backforth (Variables|Default|GetSpringArm_BackForth))
  (bind _camera_pitch_max (Variables|Default|GetCamera%20Pitch%20Max))
  (bind _camera_pitch_max_2 (Variables|Default|GetCamera%20Pitch%20Max))
  (bind _springarm_backforth_2 (Variables|Default|GetSpringArm_BackForth))
  (bind _camera_pitch_max_3 (Variables|Default|GetCamera%20Pitch%20Max))
  (bind _camera_pitch_max_4 (Variables|Default|GetCamera%20Pitch%20Max))
  (bind _returnvalue_3 (Transformation|GetWorldRotation _springarm_backforth))
  (bind _returnvalue_4 (Transformation|GetWorldRotation _springarm_backforth_2))
  (bind _returnvalue_5 (/ _returnvalue 2.0))
  (bind _returnvalue_6 (/ _returnvalue_2 2.0))
  (bind _returnvalue_7 (Math|Float|Absolute(Float) (.pitch _returnvalue_4)))
  (bind _returnvalue_8 (Math|Float|Absolute(Float) (.pitch _returnvalue_3)))
  (bind _returnvalue_9 (- _camera_pitch_max_4 _returnvalue_7))
  (bind _returnvalue_10 (+ _camera_pitch_max_2 _returnvalue_8))
  (bind _returnvalue_11 (/ _returnvalue_9 _camera_pitch_max))
  (bind _returnvalue_12 (/ _returnvalue_10 _camera_pitch_max_3))
  (bind _returnvalue_13 (* _returnvalue_5 _returnvalue_12))
  (bind _returnvalue_14 (* _returnvalue_6 _returnvalue_11))
  (bind _returnvalue_15 (Math|Trig|Cos(Radians) _returnvalue_13))
  (bind _returnvalue_16 (Math|Trig|Cos(Radians) _returnvalue_14))
  (bind _returnvalue_17 (* _returnvalue_15 -1.0))
  (bind _returnvalue_18 (* _returnvalue_16 -1.0))
  (bind _returnvalue_19 (+ _returnvalue_17 1.0))
  (bind _returnvalue_20 (+ _returnvalue_18 1.0))
  ;[0.15 0.15 0.15 0.5] true同号
  (if (>= (* (/ Input (Math|Float|Absolute(Float) Input)) (.pitch (Transformation|GetWorldRotation (Variables|Default|GetSpringArm_BackForth)))) 0.0)
    (Development|PrintString (Utilities|String|ToString(Float) _returnvalue_19))
    (return _returnvalue_19)
    (else
      (Development|PrintString (Utilities|String|ToString(Float) _returnvalue_20))
      (return _returnvalue_20))))