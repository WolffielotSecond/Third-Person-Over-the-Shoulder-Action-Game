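; Base enemy Blueprint that displays targeting feedback when it is spotted or locked.
; Spotted and unspotted events toggle a debug text, while locked and unlocked events toggle a lock widget that starts hidden.
; BeginPlay caches the widget as a head/leg lock UI, and Tick feeds it the current and maximum targeted organ values.
; A helper function returns the enemy itself.
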(event Custom|Target%20Spotted
  (Rendering|SetVisibility (Variables|Default|GetDebug%20Target%20Spotted%20Text) true false))

(event Custom|Target%20Unspotted
  (Rendering|SetVisibility (Variables|Default|GetDebug%20Target%20Spotted%20Text) false false))

(event Custom|Target%20Locked
  (Rendering|SetVisibility (Variables|Default|GetLock%20Widget) true false))

(event Custom|Target%20Unlocked
  (Rendering|SetVisibility (Variables|Default|GetLock%20Widget) false false))

(event EventTick
  (params (DeltaSeconds :type Float%20%28single-precision%29))
  (bind _organ_lock_widget (Variables|Default|GetOrgan%20Lock%20Widget)
    (:then
      (Default|OrganizeUI _organ_lock_widget (Variables|Default|GetCurrent%20Targeted%20Organ) (Variables|Default|GetMax%20Targeted%20Organ)))
    (:else)))

(event EventBeginPlay
  (bind _lock_widget (Variables|Default|GetLock%20Widget))
  (Rendering|SetVisibility _lock_widget false false)
  (bind _aswb_head_leg_lock (Utilities|Casting|CastToWB_Head_Leg_Lock (UserInterface|GetWidget _lock_widget)))
  (Variables|Default|SetOrgan%20Lock%20Widget _aswb_head_leg_lock))

(fn ConstructionScript)

(fn ReturnSelf
  (return self))