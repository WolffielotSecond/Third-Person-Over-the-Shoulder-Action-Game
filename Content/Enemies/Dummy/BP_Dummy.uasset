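; BP_Dummy is an enemy dummy that shows a lock-on widget on its currently targeted body part.
; Every Tick, after the parent's Tick, it switches on CurrentTargetedOrgan and re-attaches LockWidget to either the head or right calf socket on the Mesh.
; If OrganLockWidget is valid, it also sets the matching HEAD or LEG aim text.
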(event EventBeginPlay)

(event Collision|EventActorBeginOverlap
  (params (OtherActor :type Actor%20Object%20Reference)))

(event EventTick
  (params (DeltaSeconds :type Float%20%28single-precision%29))
  (|CallParentFunction DeltaSeconds)
  (switch int (Variables|Default|GetCurrent%20Targeted%20Organ)
    (:0
      (Transformation|AttachComponentToComponent (Variables|Default|GetLock%20Widget) (Variables|Character|GetMesh) "head" "KeepRelative" "KeepRelative" "KeepRelative" true)
      (bind _organ_lock_widget (Variables|Default|GetOrgan%20Lock%20Widget)
        (:then
          (Default|SetAimText _organ_lock_widget "HEAD"))
        (:else)))
    (:1
      (Transformation|AttachComponentToComponent (Variables|Default|GetLock%20Widget) (Variables|Character|GetMesh) "calf_r" "KeepRelative" "KeepRelative" "KeepRelative" true)
      (bind _organ_lock_widget_2 (Variables|Default|GetOrgan%20Lock%20Widget)
        (:then
          (Default|SetAimText _organ_lock_widget_2 "LEG"))
        (:else)))))

(fn ConstructionScript
  (|CallParentFunction))